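; Player character Blueprint whose only graph logic toggles a settings menu, used as the pause menu, on the IA_Pause input.
; The first press creates the BP_SettingsMenu widget and binds its Back button to the hide path; later presses reuse it by toggling visibility.
; Showing or hiding the menu also switches input mode and mouse cursor, but the game itself is never paused.
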(event `EnhancedInput|/Game/GAMR3510Assignment/Input/IA_Pause`
  (params (ActionValue :type Boolean) (ElapsedSeconds :type "Float (double-precision)") (TriggeredSeconds :type "Float (double-precision)") (InputAction :type "InputAction Object Reference" :default "/Game/GAMR3510Assignment/Input/IA_Pause.IA_Pause"))
  (bind _returnvalue (`GameplayStatics.GetPlayerController` 0))
  (:`Completed`
    (`/Engine/EditorBlueprintResources/StandardMacros.IsValid` (`self.BP_PauseMenu_Ref`)
      (:`Is Valid`
        (if (`Widget.IsVisible` (`self.BP_PauseMenu_Ref`))
          (`WidgetBlueprintLibrary.SetInputMode_GameOnly` _returnvalue :!label _label)
          (set `PlayerController.bShowMouseCursor` false _returnvalue)
          (`Widget.SetVisibility` (`self.BP_PauseMenu_Ref`) "Hidden")
          (else
            (`WidgetBlueprintLibrary.SetInputMode_GameAndUIEx` _returnvalue (stale _output_get) "DoNotLock" false :!label _label_2)
            (set `PlayerController.bShowMouseCursor` true _returnvalue)
            (`Widget.SetVisibility` (stale _output_get) "Visible"))))
      (:`Is Not Valid`
        (bind _returnvalue_2 (`|CreateWidget` "/Game/GAMR3510Assignment/UI/BP/BP_SettingsMenu.BP_SettingsMenu_C" (`GameplayStatics.GetPlayerController` 0)))
        (bind _output_get (set `self.BP_PauseMenu_Ref` _returnvalue_2))
        (add `Button.OnClicked` (`SettingsMenu.BackButton` _output_get) (delegate `OnBack`))
        (`UserWidget.AddToViewport` _output_get 0)
        (goto _label_2)))))

(event `OnBack`
  (goto _label))

(fn `UserConstructionScript`)